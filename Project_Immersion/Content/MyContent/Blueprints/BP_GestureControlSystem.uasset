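; Gesture recognition blueprint that classifies a given hand's pose from device finger-tracking data, with helpers exposing raw curl and splay values.
; GetActiveHandFingers thresholds each finger's curl into a curled flag, and per-gesture checks match exact five-finger patterns such as fist, peace and finger gun.
; GetGesture runs every check in sequence and returns ActiveGesture, which keeps its previous value when nothing matches and is not stored per hand.
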(fn `GetActiveHandFingers`
  (params (Hand :type "EHand Enum" :default "VR_LeftHand"))
  (returns (`Thumb active` :type Boolean) (`Index active` :type Boolean) (`Middle active` :type Boolean) (`Ring active` :type Boolean) (`Pinky active` :type Boolean))
  (bind _fingercurls (`SteamVRInputDeviceFunctionLibrary.GetFingerCurlsAndSplays` Hand "VR_SummaryType_FromDevice"))
  (bind (_thumb _index _middle _ring _pinky) (break `SteamVRFingerCurls` _fingercurls))
  (return (>= _thumb 0.75) (>= _index 0.75) (>= _middle 0.75) (>= _ring 0.75) (>= _pinky 0.75)))

(fn `GetGesture`
  (params (Hand :type "EHand Enum" :default "VR_LeftHand"))
  (returns (Gesture :type "/Game/MyContent/Blueprints/E_HandGestures Enum"))
  (locals (`Active gesture` :type "/Game/MyContent/Blueprints/E_HandGestures Enum"))
  (`|ExecutionSequence`
    (:`then_0`
      (bind _returnvalue (`self.IsOpen?` (`local.Hand`)))
      (if _returnvalue
        (set `local.Active gesture` "NewEnumerator9")))
    (:`then_1`
      (bind _returnvalue_2 (`self.IsPointing?` (`local.Hand`)))
      (if _returnvalue_2
        (set `local.Active gesture` "NewEnumerator1")))
    (:`then_2`
      (bind _returnvalue_3 (`self.IsThumbsUp?` (`local.Hand`)))
      (if _returnvalue_3
        (set `local.Active gesture` "NewEnumerator2")))
    (:`then_3`
      (bind _returnvalue_4 (`self.IsFist?` (`local.Hand`)))
      (if _returnvalue_4
        (set `local.Active gesture` "NewEnumerator3")))
    (:`then_4`
      (bind _returnvalue_5 (`self.IsRockon?` (`local.Hand`)))
      (if _returnvalue_5
        (set `local.Active gesture` "NewEnumerator4")))
    (:`then_5`
      (bind _returnvalue_6 (`self.IsGotem?` (`local.Hand`)))
      (if _returnvalue_6
        (set `local.Active gesture` "NewEnumerator5")))
    (:`then_6`
      (bind _returnvalue_7 (`self.IsTelephone?` (`local.Hand`)))
      (if _returnvalue_7
        (set `local.Active gesture` "NewEnumerator6")))
    (:`then_7`
      (bind _returnvalue_8 (`self.IsPeace?` (`local.Hand`)))
      (if _returnvalue_8
        (set `local.Active gesture` "NewEnumerator7")))
    (:`then_8`
      (bind _returnvalue_9 (`self.IsFingerGun` (`local.Hand`)))
      (if _returnvalue_9
        (set `local.Active gesture` "NewEnumerator8")))
    (:`then_9`
      (return (`local.Active gesture`)))))

(fn `GetHandFingerCurls`
  (params (Hand :type "EHand Enum" :default "VR_LeftHand"))
  (returns (Thumb :type "Float (single-precision)") (Index :type "Float (single-precision)") (Middle :type "Float (single-precision)") (Ring :type "Float (single-precision)") (Pinky :type "Float (single-precision)"))
  (bind _fingercurls (`SteamVRInputDeviceFunctionLibrary.GetFingerCurlsAndSplays` Hand "VR_SummaryType_FromDevice"))
  (bind (_thumb _index _middle _ring _pinky) (break `SteamVRFingerCurls` _fingercurls))
  (return _thumb _index _middle _ring _pinky))

(fn `GetHandFingerSplays`
  (params (Hand :type "EHand Enum" :default "VR_LeftHand"))
  (returns (`Thumb Index` :type "Float (single-precision)") (`Index Middle` :type "Float (single-precision)") (`Middle Ring` :type "Float (single-precision)") (`Ring Pinky` :type "Float (single-precision)"))
  (bind (_fingercurls _fingersplays) (`SteamVRInputDeviceFunctionLibrary.GetFingerCurlsAndSplays` Hand "VR_SummaryType_FromDevice"))
  (bind (_thumb_index _index_middle _middle_ring _ring_pinky) (break `SteamVRFingerSplays` _fingersplays))
  (return _thumb_index _index_middle _middle_ring _ring_pinky))

(fn `IsFingerGun`
  (params (Hand :type "EHand Enum" :default "VR_LeftHand"))
  (returns (ReturnValue :type Boolean))
  (bind (_thumb_active _index_active _middle_active _ring_active _pinky_active) (`self.GetActiveHandFingers` Hand))
  (return (and (== _thumb_active false) (== _index_active false) (== _middle_active true) (== _ring_active true) (== _pinky_active true))))

(fn `IsFist?`
  (params (Hand :type "EHand Enum" :default "VR_LeftHand"))
  (returns (ReturnValue :type Boolean))
  (bind (_thumb_active _index_active _middle_active _ring_active _pinky_active) (`self.GetActiveHandFingers` Hand))
  (return (and (== _thumb_active true) (== _index_active true) (== _middle_active true) (== _ring_active true) (== _pinky_active true))))

(fn `IsGotem?`
  (params (Hand :type "EHand Enum" :default "VR_LeftHand"))
  (returns (ReturnValue :type Boolean))
  (bind (_thumb_active _index_active _middle_active _ring_active _pinky_active) (`self.GetActiveHandFingers` Hand))
  (return (and (== _thumb_active true) (== _index_active true) (== _middle_active false) (== _ring_active false) (== _pinky_active false))))

(fn `IsOpen?`
  (params (Hand :type "EHand Enum" :default "VR_LeftHand"))
  (returns (ReturnValue :type Boolean))
  (bind (_thumb_active _index_active _middle_active _ring_active _pinky_active) (`self.GetActiveHandFingers` Hand))
  (return (and (== _thumb_active false) (== _index_active false) (== _middle_active false) (== _ring_active false) (== _pinky_active false))))

(fn `IsPeace?`
  (params (Hand :type "EHand Enum" :default "VR_LeftHand"))
  (returns (ReturnValue :type Boolean))
  (bind (_thumb_active _index_active _middle_active _ring_active _pinky_active) (`self.GetActiveHandFingers` Hand))
  (return (and (== _thumb_active true) (== _index_active false) (== _middle_active false) (== _ring_active true) (== _pinky_active true))))

(fn `IsPointing?`
  (params (Hand :type "EHand Enum" :default "VR_LeftHand"))
  (returns (ReturnValue :type Boolean))
  (bind (_thumb_active _index_active _middle_active _ring_active _pinky_active) (`self.GetActiveHandFingers` Hand))
  (return (and (== _thumb_active true) (== _index_active false) (== _middle_active true) (== _ring_active true) (== _pinky_active true))))

(fn `IsRockon?`
  (params (Hand :type "EHand Enum" :default "VR_LeftHand"))
  (returns (ReturnValue :type Boolean))
  (bind (_thumb_active _index_active _middle_active _ring_active _pinky_active) (`self.GetActiveHandFingers` Hand))
  (return (and (== _thumb_active true) (== _index_active false) (== _middle_active true) (== _ring_active true) (== _pinky_active false))))

(fn `IsTelephone?`
  (params (Hand :type "EHand Enum" :default "VR_LeftHand"))
  (returns (ReturnValue :type Boolean))
  (bind (_thumb_active _index_active _middle_active _ring_active _pinky_active) (`self.GetActiveHandFingers` Hand))
  (return (and (== _thumb_active false) (== _index_active true) (== _middle_active true) (== _ring_active true) (== _pinky_active false))))

(fn `IsThumbsUp?`
  (params (Hand :type "EHand Enum" :default "VR_LeftHand"))
  (returns (ReturnValue :type Boolean))
  (bind (_thumb_active _index_active _middle_active _ring_active _pinky_active) (`self.GetActiveHandFingers` Hand))
  (return (and (== _thumb_active false) (== _index_active true) (== _middle_active true) (== _ring_active true) (== _pinky_active true))))