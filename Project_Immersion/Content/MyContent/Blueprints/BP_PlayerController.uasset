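; Player controller that drives the BP_Player pawn's movement and turning from axis input.
; It caches the pawn on BeginPlay and checks that reference before each input.
; MoveLeft axes move the pawn at half scale along the X and Y components of the camera's right and forward vectors.
; MoveRight_X yaws the whole actor by LookRotationSpeed, with no pitch input handled.
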(event `self.ReceiveBeginPlay`
  (bind _asbp_player (cast `/Game/MyContent/Blueprints/BP_Player` (`GameplayStatics.GetPlayerPawn` 0)))
  (set `self.Player ref` _asbp_player))

(event `InputAxis|MoveLeft_X`
  (params (AxisValue :type "Float (single-precision)"))
  ;[1 1 1] Movement
  (bind _player_ref (`self.Player ref`)
    (:`then`
      (bind (_returnvalue_x _returnvalue_y) (`KismetMathLibrary.BreakVector` (`SceneComponent.GetRightVector` (`/Game/MyContent/Blueprints/BP_Player.Camera` _player_ref))))
      (`Pawn.AddMovementInput` _player_ref (`KismetMathLibrary.MakeVector` _returnvalue_x _returnvalue_y) (* AxisValue 0.5) false))
    (:`else`)))

(event `InputAxis|MoveLeft_Y`
  (params (AxisValue :type "Float (single-precision)"))
  ;[1 1 1] Movement
  (bind _player_ref (`self.Player ref`)
    (:`then`
      (bind (_returnvalue_x _returnvalue_y) (`KismetMathLibrary.BreakVector` (`SceneComponent.GetForwardVector` (`/Game/MyContent/Blueprints/BP_Player.Camera` _player_ref))))
      (`Pawn.AddMovementInput` _player_ref (`KismetMathLibrary.MakeVector` _returnvalue_x _returnvalue_y) (* AxisValue 0.5) false))
    (:`else`)))

(event `InputAxis|MoveRight_X`
  (params (AxisValue :type "Float (single-precision)"))
  ;[1 1 1] Looking
  (bind _player_ref (`self.Player ref`)
    (:`then`
      (`self.K2_AddActorWorldRotation` _player_ref (`KismetMathLibrary.MakeRotator` 0.0 0.0 (* AxisValue (`self.Look rotation speed`))) false false))
    (:`else`)))

(fn `UserConstructionScript`)