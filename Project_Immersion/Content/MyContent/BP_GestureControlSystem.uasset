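; Gesture control component for a VR motion controller pawn that exposes per-finger hand tracking data.
; Two helper functions break the animation-based skeletal summary for a given hand into five finger curl values and four splay values between adjacent fingers.
; On BeginPlay it prints an activation message and, through an always-true branch, puts a gesture debug widget on the owning pawn's HUD.
; No gesture recognition happens here, and Tick is empty.
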(event `self.ReceiveTick`
  (params (DeltaSeconds :type "Float (single-precision)")))

(event `self.ReceiveBeginPlay`
  ;[0.1274 1 0] Set player HUD to debug HUD if "Show Debug UI" is enabled
  (`KismetSystemLibrary.PrintString` "GESTURE CONTROL SYSTEM ACTIVE!" true true (struct :`R` 0.127447 :`G` 1.0 :`A` 1.0))
  (if true
    (bind _returnvalue (`|CreateWidget` "/Game/MyContent/UI_GestureControlDebug.UI_GestureControlDebug_C" (`GameplayStatics.GetPlayerController` 0)))
    (bind _asmotion_controller_pawn (cast `/Game/EpicTemplates/VRTemplate/Blueprints/MotionControllerPawn` (`self.GetOwner`)))
    (`WidgetComponent.SetWidget` (`/Game/EpicTemplates/VRTemplate/Blueprints/MotionControllerPawn.HUD` _asmotion_controller_pawn) _returnvalue)))

(fn `GetHandFingerCurls`
  (params (Hand :type "EHand Enum" :default "VR_LeftHand"))
  (returns (Thumb :type "Float (single-precision)") (Index :type "Float (single-precision)") (Middle :type "Float (single-precision)") (Ring :type "Float (single-precision)") (Pinky :type "Float (single-precision)"))
  (bind _fingercurls (`SteamVRInputDeviceFunctionLibrary.GetFingerCurlsAndSplays` Hand))
  (bind (_thumb _index _middle _ring _pinky) (break `SteamVRFingerCurls` _fingercurls))
  (return _thumb _index _middle _ring _pinky))

(fn `GetHandFingerSplays`
  (params (Hand :type "EHand Enum" :default "VR_LeftHand"))
  (returns (`Thumb Index` :type "Float (single-precision)") (`Index Middle` :type "Float (single-precision)") (`Middle Ring` :type "Float (single-precision)") (`Ring Pinky` :type "Float (single-precision)"))
  (bind (_fingercurls _fingersplays) (`SteamVRInputDeviceFunctionLibrary.GetFingerCurlsAndSplays` Hand))
  (bind (_thumb_index _index_middle _middle_ring _ring_pinky) (break `SteamVRFingerSplays` _fingersplays))
  (return _thumb_index _index_middle _middle_ring _ring_pinky))