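; Player controller that translates movement and look axis inputs into actions on BP_Player.
; On BeginPlay it casts and caches the player pawn as PlayerRef.
; MoveLeft axes add half-scale movement input along the X and Y components of the camera's forward and right vectors, so movement follows camera heading.
; MoveRight_X yaws the whole pawn by LookRotationSpeed, with no pitch input and no delta-time scaling.
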(event `self.ReceiveBeginPlay`
  (bind _asbp_player (cast `/Game/MyContent/BP_Player` (`GameplayStatics.GetPlayerPawn` 0)))
  (set `self.Player ref` _asbp_player))

(event `InputAxis|MoveLeft_X`
  (params (AxisValue :type "Float (single-precision)"))
  (bind _player_ref (`self.Player ref`))
  (bind (_returnvalue_x _returnvalue_y) (`KismetMathLibrary.BreakVector` (`SceneComponent.GetRightVector` (`/Game/MyContent/BP_Player.Camera` _player_ref))))
  ;[1 1 1] Movement
  (`Pawn.AddMovementInput` _player_ref (`KismetMathLibrary.MakeVector` _returnvalue_x _returnvalue_y) (* AxisValue 0.5) false))

(event `InputAxis|MoveLeft_Y`
  (params (AxisValue :type "Float (single-precision)"))
  (bind _player_ref (`self.Player ref`))
  (bind (_returnvalue_x _returnvalue_y) (`KismetMathLibrary.BreakVector` (`SceneComponent.GetForwardVector` (`/Game/MyContent/BP_Player.Camera` _player_ref))))
  ;[1 1 1] Movement
  (`Pawn.AddMovementInput` _player_ref (`KismetMathLibrary.MakeVector` _returnvalue_x _returnvalue_y) (* AxisValue 0.5) false))

(event `InputAxis|MoveRight_X`
  (params (AxisValue :type "Float (single-precision)"))
  ;[1 1 1] Looking
  (`self.K2_AddActorWorldRotation` (`self.Player ref`) (`KismetMathLibrary.MakeRotator` 0.0 0.0 (* AxisValue (`self.Look rotation speed`))) false false))

(fn `UserConstructionScript`)